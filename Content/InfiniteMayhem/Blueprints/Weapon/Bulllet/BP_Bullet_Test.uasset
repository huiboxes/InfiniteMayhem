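; Test bullet projectile that leaves a temporary impact decal, plays surface-specific effects and destroys itself when its collision sphere hits something.
; PlayHitObjectFX runs a zero-length sphere trace at the hit point to read the physical surface, then picks a particle and sound, defaulting to gravel/dirt.
; The emitter and sound calls have no location input set.
; Impulse logic for physics-simulating components exists but is unconnected.
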(event `self.ReceiveBeginPlay`)

(event `self.SphereCollision.OnComponentHit`
  (params (HitComponent :type "PrimitiveComponent Object Reference") (OtherActor :type "Actor Object Reference") (OtherComp :type "PrimitiveComponent Object Reference") (NormalImpulse :type "Vector Structure") (Hit :type "HitResult Structure (by ref)"))
  (bind (_bblockinghit _binitialoverlap _time _distance _location _impactpoint _normal) (`GameplayStatics.BreakHitResult` Hit))
  (`GameplayStatics.SpawnDecalAtLocation` "/Game/InfiniteMayhem/Materials/Bullet_Impact_Decal.Bullet_Impact_Decal" (7.0 0.0 0.0) _location (`KismetMathLibrary.Conv_VectorToRotator` _normal) 20.0)
  (`self.Play Hit Object FX` Hit)
  (`|ExecutionSequence`
    (:`then_1`
      (`self.K2_DestroyActor`))))

(fn `Play Hit Object FX`
  (params (Hit :type "HitResult Structure"))
  (bind (_bblockinghit _binitialoverlap _time _distance _location _impactpoint _normal) (`GameplayStatics.BreakHitResult` Hit))
  (bind _returnvalue (`KismetMathLibrary.Conv_VectorToRotator` _normal))
  (bind _outhit (`KismetSystemLibrary.SphereTraceSingle` _location _location 10.0 "TraceTypeQuery3"))
  (switch `EPhysicalSurface` (`GameplayStatics.GetSurfaceType` _outhit)
    (:`SurfaceType_Default`
      (`GameplayStatics.SpawnEmitterAtLocation` "/Game/InfiniteMayhem/FX/Particles/GunImpacts1/Particles/P_ImpactDirt.P_ImpactDirt" (0.0 0.0 0.0) _returnvalue (0.6 0.6 0.6) :!label _label)
      (`GameplayStatics.PlaySoundAtLocation` "/Game/InfiniteMayhem/Sounds/BulletImpact/Gravel/bullet_impact_gravel_01_Cue.bullet_impact_gravel_01_Cue" (0.0 0.0 0.0) (struct) 1.0 1.0 0.0 null null null))
    (:`SurfaceType1`
      (`GameplayStatics.SpawnEmitterAtLocation` "/Game/InfiniteMayhem/FX/Particles/GunImpacts1/Particles/P_ImpactMetal.P_ImpactMetal" (0.0 0.0 0.0) _returnvalue (0.6 0.6 0.6))
      (`GameplayStatics.PlaySoundAtLocation` "/Game/InfiniteMayhem/Sounds/BulletImpact/Metal/bullet_impact_metal_heavy_01_Cue.bullet_impact_metal_heavy_01_Cue" (0.0 0.0 0.0) (struct) 1.0 1.0 0.0 null null null))
    (:`SurfaceType2`
      (goto _label))
    (:`SurfaceType3`
      (`GameplayStatics.SpawnEmitterAtLocation` "/Game/InfiniteMayhem/FX/Particles/GunImpacts1/Particles/P_ImpactConcrete.P_ImpactConcrete" (0.0 0.0 0.0) _returnvalue)
      (`GameplayStatics.PlaySoundAtLocation` "/Game/InfiniteMayhem/Sounds/BulletImpact/Concrete/bullet_impact_concrete_brick_01_Cue.bullet_impact_concrete_brick_01_Cue" (0.0 0.0 0.0) (struct) 1.0 1.0 0.0 null null null))
    (:`SurfaceType4`
      (`GameplayStatics.SpawnEmitterAtLocation` "/Game/InfiniteMayhem/FX/Particles/GunImpacts1/Particles/P_ImpactWood.P_ImpactWood" (0.0 0.0 0.0) _returnvalue (0.6 0.6 0.6))
      (`GameplayStatics.PlaySoundAtLocation` "/Game/InfiniteMayhem/Sounds/BulletImpact/Wood/bullet_impact_wood_heavy_01_Cue.bullet_impact_wood_heavy_01_Cue" (0.0 0.0 0.0) (struct) 1.0 1.0 0.0 null null null))
    (:`SurfaceType5`
      (`GameplayStatics.SpawnEmitterAtLocation` "/Game/InfiniteMayhem/FX/Particles/GunImpacts1/Particles/P_ImpactRock.P_ImpactRock" (0.0 0.0 0.0) _returnvalue (0.6 0.6 0.6))
      (`GameplayStatics.PlaySoundAtLocation` "/Game/InfiniteMayhem/Sounds/BulletImpact/Rock/bullet_impact_rock_01_Cue.bullet_impact_rock_01_Cue" (0.0 0.0 0.0) (struct) 1.0 1.0 0.0 null null null))
    (:`SurfaceType6`
      (`GameplayStatics.SpawnEmitterAtLocation` "/Game/InfiniteMayhem/FX/Particles/GunImpacts1/Particles/P_ImpactGrass.P_ImpactGrass" (0.0 0.0 0.0) _returnvalue (0.6 0.6 0.6))
      (`GameplayStatics.PlaySoundAtLocation` "/Game/InfiniteMayhem/Sounds/BulletImpact/Concrete/bullet_impact_concrete_brick_01_Cue.bullet_impact_concrete_brick_01_Cue" (0.0 0.0 0.0) (struct) 1.0 1.0 0.0 null null null))))

(fn `UserConstructionScript`)