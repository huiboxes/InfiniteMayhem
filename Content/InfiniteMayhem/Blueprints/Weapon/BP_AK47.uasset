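; AK-47 weapon Blueprint that adds camera recoil when the weapon fires.
; BeginPlay binds the OnWeaponFire dispatcher to a handler that restarts a recoil timeline from the beginning.
; The forward pass feeds scaled pitch and random side-to-side yaw into player controller 0.
; On finish the timeline reverses, applying weaker opposite pitch for partial recovery, with no yaw correction.
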(event `WeaponFireHandle`
  (bind _returnvalue (`GameplayStatics.GetPlayerController` 0))
  (bind _recoilyaw (`self.RecoilYaw`))
  (bind (_direction _alpha) (`Timeline|RecoilTimeline` :!via `PlayFromStart` :!label _label)
    (:`Update`
      (switch `ETimelineDirection` _direction
        (:`Forward`
          (bind _returnvalue_2 (`KismetMathLibrary.Lerp` 0.0 (`self.RecoilPitch`) _alpha))
          (`PlayerController.AddPitchInput` _returnvalue _returnvalue_2)
          (`PlayerController.AddYawInput` _returnvalue (`KismetMathLibrary.RandomFloatInRange` (* _recoilyaw -1.0) _recoilyaw)))
        (:`Backward`
          (`PlayerController.AddPitchInput` _returnvalue (* _returnvalue_2 -0.8)))))
    (:`Finished`
      (`self.RecoilRebouce`))))

(event `RecoilRebouce`
  (goto _label :!via `Reverse`))

(event `self.ReceiveBeginPlay`
  (add `self.OnWeaponFire` (delegate `WeaponFireHandle`)))

(fn `UserConstructionScript`)