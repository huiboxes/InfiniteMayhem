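; BP_Weapon is a weapon actor that fires bullets automatically between start and stop events.
; StartFire waits a precast delay, fires once, then runs a looping timer at the firing rate until StopFire clears it.
; Each shot spawns a scaled-down BulletClass actor plus shell-eject and muzzle emitters, with only the shell placed at the Arrow component.
; The fire animation and muzzle socket lookups are not connected.
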(event `Firing`
  (bind (_returnvalue_location _returnvalue_rotation) (`KismetMathLibrary.BreakTransform` (`SceneComponent.K2_GetComponentToWorld` (`self.Arrow`))))
  (`|SpawnActorFromClass` (`self.Bullet_Class`) (`KismetMathLibrary.MakeTransform` (0.0 0.0 0.0) (struct) (0.2 0.2 0.2)) "Undefined" "OverrideRootScale" null null)
  (`GameplayStatics.SpawnEmitterAtLocation` "/Game/InfiniteMayhem/FX/Particles/Weapons/Effects/ParticleSystems/Ammo_Shell_Reject2.Ammo_Shell_Reject2" _returnvalue_location _returnvalue_rotation)
  (`GameplayStatics.SpawnEmitterAtLocation` "/Game/InfiniteMayhem/FX/Particles/MuzzleFlame/VFX/Particle_Systems/Muzzle_01.Muzzle_01" (0.0 0.0 0.0) (struct) (0.4 0.4 0.4)))

(event `StartFire`
  (`KismetSystemLibrary.Delay` (`self.PrecastTime`))
  (`self.Firing`)
  (bind _returnvalue (`KismetSystemLibrary.K2_SetTimerDelegate` (delegate `Firing`) (`self.FiringRate`) true)))

(event `StopFire`
  (`KismetSystemLibrary.K2_ClearAndInvalidateTimerHandle` (stale `StartFire` _returnvalue)))

(fn `UserConstructionScript`)