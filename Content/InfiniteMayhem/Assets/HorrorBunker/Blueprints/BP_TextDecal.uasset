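; BP_TextDecal is a configurable decal actor for the HorrorBunker asset set, with per-instance appearance.
; Its construction script creates a dynamic material on the Decal and passes in the actor's variables for atlas texture, columns, UV coordinates, offsets, colour, roughness and wear.
; The UpperLeftCornerV parameter is fed from the UpperLeftCornerU variable, and no UpperLeftCornerU parameter is set.
; The event graph holds only disabled stubs, so nothing runs during play.
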(fn `UserConstructionScript`
  (bind _returnvalue (`DecalComponent.CreateDynamicMaterialInstance` (`self.Decal`)))
  (`MaterialInstanceDynamic.SetScalarParameterValue` _returnvalue "UpperLeftCornerV" (`self.UpperLeftCornerU`))
  (`MaterialInstanceDynamic.SetScalarParameterValue` _returnvalue "TexCoordU" (`self.TexCoordU`))
  (`MaterialInstanceDynamic.SetScalarParameterValue` _returnvalue "TexCoordV" (`self.TexCoordV`))
  (`MaterialInstanceDynamic.SetVectorParameterValue` _returnvalue "Colour" (`self.Colour`))
  (`MaterialInstanceDynamic.SetScalarParameterValue` _returnvalue "OffsetX" (`self.Offset X`))
  (`MaterialInstanceDynamic.SetScalarParameterValue` _returnvalue "OffsetY" (`self.Offset Y`))
  (`MaterialInstanceDynamic.SetScalarParameterValue` _returnvalue "Roughness Strength" (`self.Roughness Strength`))
  (`MaterialInstanceDynamic.SetScalarParameterValue` _returnvalue "Wear Strength" (`self.Wear Strength`))
  (`MaterialInstanceDynamic.SetTextureParameterValue` _returnvalue "DecalSet" (`self.Decal Set`))
  (`MaterialInstanceDynamic.SetScalarParameterValue` _returnvalue "Number of Coloums" (`self.Number of Coloums`)))